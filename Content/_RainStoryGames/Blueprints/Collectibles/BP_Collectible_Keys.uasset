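; BP_Collectible_Keys is a key pickup Blueprint in the game's collectibles set.
; Its CalculateCollectibles event adds one to the Keys count and adds ScoreValue to the Score, both stored on ControllerReference.
; The event graph holds no other active logic, and the construction script only calls its parent.
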(event `self.CalculateCollectibles`
  (bind _controllerreference (`self.ControllerReference`))
  (set `/Game/_RainStoryGames/Blueprints/PC_Rainstory_Platformer.Keys` (+ (`/Game/_RainStoryGames/Blueprints/PC_Rainstory_Platformer.Keys` _controllerreference) 1) _controllerreference)
  (set `/Game/_RainStoryGames/Blueprints/PC_Rainstory_Platformer.Score` (+ (`/Game/_RainStoryGames/Blueprints/PC_Rainstory_Platformer.Score` _controllerreference) (`self.ScoreValue`)) _controllerreference))

(fn `UserConstructionScript`
  (`parent.UserConstructionScript`))