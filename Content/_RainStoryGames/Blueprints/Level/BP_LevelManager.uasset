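; Level manager actor for the Rainstory platformer that starts the level's music and optional timer or countdown, and acts as the exit to the next level.
; When the player overlaps its sphere, it compares coin and star counts on the player controller and opens the next level, requiring completion only if CollectAll is set.
; Unmet objectives play a sound and typewriter dialogue, guarded against repeats until the text is removed after a delay.
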(event `self.ReceiveBeginPlay`
  (`|ExecutionSequence`
    (:`then_0`
      (bind _aspc_rainstory_platformer (cast `/Game/_RainStoryGames/Blueprints/PC_Rainstory_Platformer` (`GameplayStatics.GetPlayerController` 0)))
      (set `self.ControllerReference` _aspc_rainstory_platformer)
      (`self.SetCountdownMode`)
      (`self.SetTimerMode`))
    (:`then_1`
      (`GameplayStatics.PlaySound2D` (`self.LevelMusic`) 1.0 1.0 0.0 null null))))

(event `self.Sphere.OnComponentBeginOverlap`
  (params (OverlappedComponent :type "PrimitiveComponent Object Reference") (OtherActor :type "Actor Object Reference") (OtherComp :type "PrimitiveComponent Object Reference") (OtherBodyIndex :type Integer) (bFromSweep :type Boolean) (SweepResult :type "HitResult Structure (by ref)"))
  (if (`self.ActorHasTag` OtherActor "Player")
    (`self.CheckObjectives`)
    (if (`self.CollectAll?`)
      (if (`self.ObjectivesComplete`)
        (`GameplayStatics.OpenLevel` (`self.NextLevel`) :!label _label))
      (else
        (goto _label)))))

(event `CheckObjectives`
  (bind _controllerreference (`self.ControllerReference`))
  ;[1 1 1] Checks if you have picked all the collectibles in the level
  (if (and (== (`/Game/_RainStoryGames/Blueprints/PC_Rainstory_Platformer.Coins` _controllerreference) (`/Game/_RainStoryGames/Blueprints/PC_Rainstory_Platformer.Coins_Count` _controllerreference)) (== (`/Game/_RainStoryGames/Blueprints/PC_Rainstory_Platformer.Stars` _controllerreference) (`/Game/_RainStoryGames/Blueprints/PC_Rainstory_Platformer.Stars_Count` _controllerreference)))
    (set `self.ObjectivesComplete` true)
    (else
      (`self.CustomDialogue`))))

(event `SetCountdownMode`
  ;[1 1 1] Choose if you want a timer or countdown for your level
  (if (and (`self.CountdownMode`) (not (`self.TimerMode`)))
    (`/Game/_RainStoryGames/Blueprints/PC_Rainstory_Platformer.StartCountdown` (`self.ControllerReference`))))

(event `SetTimerMode`
  ;[1 1 1] Choose if you want a timer or countdown for your level
  (if (and (`self.TimerMode`) (not (`self.CountdownMode`)))
    (`/Game/_RainStoryGames/Blueprints/PC_Rainstory_Platformer.StartTimer` (`self.ControllerReference`))))

(event `CustomDialogue`
  (if (`self.DialogueOver`)
    (set `self.DialogueOver` false)
    (`GameplayStatics.PlaySoundAtLocation` (`self.Sound`) (`SceneComponent.K2_GetComponentLocation` (`self.DefaultSceneRoot`)) (struct) 1.0 1.0 0.0 null null null null)
    (bind _aspc_rainstory_platformer (cast `/Game/_RainStoryGames/Blueprints/PC_Rainstory_Platformer` (`GameplayStatics.GetPlayerController` 0)))
    (bind _returnvalue (`|CreateWidget` "/Game/_RainStoryGames/Blueprints/UI/Typewriter/UI_Typewriter.UI_Typewriter_C" _aspc_rainstory_platformer (`self.Characters Per Second`) (`self.TextColor`)))
    (`UserWidget.AddToViewport` _returnvalue 0)
    (`/Game/_RainStoryGames/Blueprints/UI/Typewriter/UI_Typewriter.Write` _returnvalue (`self.WriteText`))
    (add `/Game/_RainStoryGames/Blueprints/UI/Typewriter/UI_Typewriter.FinishedWriting` _returnvalue (delegate `CustomEvent_3`))))

(event `CustomEvent_3`
  (`KismetSystemLibrary.Delay` (`self.RemoveAfter`))
  (`Widget.RemoveFromParent` (stale `CustomDialogue` _returnvalue))
  (set `self.DialogueOver` true))

(fn `UserConstructionScript`)